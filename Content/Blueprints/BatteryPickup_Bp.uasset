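; Battery pickup Blueprint that adds electrical effects to its parent's collection and light-destroy events.
; On collection, an electricity arc beam attached to the mesh re-targets the player's spine socket on a short repeating delay loop, while the parent handler runs after a brief pause.
; LightDestroy plays the arc, then a second particle effect, each followed by a delay before calling the parent handler.
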(event EventLightDestroy
  (Effects|SpawnEmitterAttached "/Game/ExampleContent/Effects/ParticleSystems/P_electricity_arc.P_electricity_arc" (Variables|Default|GetPickupMesh) "None" "0, 0, 0" "0, 0, 0" "1.000000,1.000000,1.000000" "SnapToTargetIncludingScale")
  (Utilities|FlowControl|Delay 3.0)
  (Effects|SpawnEmitterAttached "/Engine/Tutorial/SubEditors/TutorialAssets/TutorialParticleSystem.TutorialParticleSystem" (Variables|Default|GetPickupMesh) "None" "0, 0, 0" "0, 0, 0" "1.000000,1.000000,1.000000" "SnapToTargetIncludingScale")
  (Utilities|FlowControl|Delay 2.0)
  (|CallParentFunction))

(event EventWasCollected
  (bind _returnvalue (Effects|SpawnEmitterAttached "/Game/ExampleContent/Effects/ParticleSystems/P_electricity_arc.P_electricity_arc" (Variables|Default|GetPickupMesh) "None" "0, 0, 0" "0, 0, 0" "1.000000,1.000000,1.000000" "SnapToTargetIncludingScale"))
  (Class|ParticleSystemComponent|SetBeamTargetPoint _returnvalue 0 (Transformation|GetSocketLocation (Variables|/Script/Engine.Character|GetMesh (Game|GetPlayerCharacter 0)) "spine_02") :!label _label)
  (Utilities|FlowControl|Sequence
    (:then_0
      (Utilities|FlowControl|Delay 1.0)
      (|CallParentFunction))
    (:then_1
      (Utilities|FlowControl|Delay 0.1)
      (goto _label))))

(fn ConstructionScript)